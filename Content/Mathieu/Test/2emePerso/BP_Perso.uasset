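; Test AI character that walks up to the player's top-down character on BeginPlay and plays a caressing animation.
; An AI MoveTo targets the player; on success it starts the intro animation and immediately enters a delayed loop.
; While ContinueCaresser is true, the CaresseDorG flag flips to alternate forward and reverse stroke animations played directly on the mesh, with debug prints.
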(event `self.ReceiveBeginPlay`
  (bind _asbp_top_down_character (cast `/Game/TopDown/Blueprints/BP_TopDownCharacter` (`GameplayStatics.GetPlayerCharacter` 0)))
  (set `self.PP` _asbp_top_down_character)
  (`self.GoCaresser`))

(event `GoCaresser`
  (`|AIMoveTo` self (0.0 0.0 0.0) (`self.PP`) 250.0
    (:`OnSuccess`
      (`SkeletalMeshComponent.PlayAnimation` (`self.Mesh`) "/Game/Mathieu/Test/Animation/BlueSoldier_Female_Anim_CharacterArmature_CaresserStart.BlueSoldier_Female_Anim_CharacterArmature_CaresserStart" false)
      (if (`self.ContinueCaresser?`) :!label _label
        (if (`self.CaresseDorG?`)
          (bind _output_get (set `self.CaresseDorG?` false))
          (`KismetSystemLibrary.PrintString` (`KismetStringLibrary.Conv_BoolToString` _output_get))
          (`SkeletalMeshComponent.PlayAnimation` (`self.Mesh`) "/Game/Mathieu/Test/Animation/BlueSoldier_Female_Anim_CharacterArmature_Caresser.BlueSoldier_Female_Anim_CharacterArmature_Caresser" false)
          (else
            (bind _output_get_2 (set `self.CaresseDorG?` true))
            (`KismetSystemLibrary.PrintString` (`KismetStringLibrary.Conv_BoolToString` _output_get_2))
            (`SkeletalMeshComponent.PlayAnimation` (`self.Mesh`) "/Game/Mathieu/Test/Animation/BlueSoldier_Female_Anim_CharacterArmature_Caresser_Reverse.BlueSoldier_Female_Anim_CharacterArmature_Caresser_Reverse" false)))
        (`KismetSystemLibrary.Delay` 0.38)
        (goto _label)))))

(fn `UserConstructionScript`)