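; Quick-time event actor for a human interaction ("Caresse"), where the player answers timed left/right click prompts.
; StartQte shows a background, then a recursive, delayed AddInput reads each QTEEnum step from DT_QTE1 and spawns an animated WB_Qte.
; Tick keeps the first queued widget active.
; WinQte and LooseQte clear the UI and trigger the character's reaction, with the player dancing on a win.
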(event `self.ReceiveBeginPlay`
  (bind _asbp_top_down_character (cast `/Game/TopDown/Blueprints/BP_TopDownCharacter` (`GameplayStatics.GetPlayerCharacter` 0)))
  (set `self.PP` _asbp_top_down_character))

(event `AddInput`
  (bind _returnvalue (`|GetDataTableRow` "/Game/Mathieu/InteractHuman/DT_QTE1.DT_QTE1" (`KismetStringLibrary.Conv_StringToName` (`|GetEnumeratorNameAsString` (`|GetArrayItem` (`self.QTE_Enum`) (`self.WhichInput?`)))))
    (:`then`
      (if (and (>= (`KismetArrayLibrary.Array_Length` (`self.QTE_Enum`)) (`self.WhichInput?`)) (`self.Continue`))
        (bind _laswidget_ (`self.LastWidget`))
        (`self.AugmentInput`)
        (bind (_input _delay _speed) (break `/Game/Mathieu/InteractHuman/Struct_QTE1` _returnvalue))
        (bind (_image _tord) (`self.CheckInput` _input))
        (`self.CreateWidget` _image _tord _speed _laswidget_)
        (`KismetSystemLibrary.Delay` _delay)
        (`self.AddInput`)))))

(event `StartQte`
  (params (Perso :type "/Game/Mathieu/Test/2emePerso/BP_Perso Object Reference"))
  (set `self.Perso` Perso)
  (set `/Game/TopDown/Blueprints/BP_TopDownCharacter.In QTE` true (`self.PP`))
  (set `self.Continue` true)
  (`/Engine/EditorBlueprintResources/StandardMacros.DoOnce` false
    (:`Completed`
      (bind _returnvalue (`|CreateWidget` "/Game/Mathieu/InteractHuman/WB_BackgroundQTE.WB_BackgroundQTE_C"))
      (bind _output_get (set `self.Background` _returnvalue))
      (`UserWidget.AddToViewport` _output_get 0)
      (`self.AddInput`))))

(event `self.ReceiveTick`
  (params (DeltaSeconds :type "Float (single-precision)"))
  (bind _output (`|GetArrayItem` (`self.WidgetActif?`)))
  (`/Engine/EditorBlueprintResources/StandardMacros.IsValid` _output
    (:`Is Valid`
      (set `/Game/Mathieu/InteractHuman/WB_Qte.IsActive?` true _output))))

(event `LooseQte`
  (set `self.Continue` false)
  (`Widget.RemoveFromParent` (`self.Background`))
  (`/Game/Mathieu/Test/2emePerso/BP_Perso.SeFaitTabass` (`self.Perso`))
  (for _array_element (`self.WidgetActif?`)
    (`Widget.RemoveFromParent` _array_element)))

(event `WinQte`
  (bind _pp (`self.PP`))
  (set `self.Continue` false)
  (`Widget.RemoveFromParent` (`self.Background`))
  (`/Game/Mathieu/Test/2emePerso/BP_Perso.BeHappy` (`self.Perso`))
  (set `/Game/TopDown/Blueprints/BP_TopDownCharacter.In QTE` false _pp)
  (`/Game/TopDown/Blueprints/BP_TopDownCharacter.Dance` _pp)
  (for _array_element (`self.WidgetActif?`)
    (`Widget.RemoveFromParent` _array_element)))

(fn `AugmentInput`
  (bind _result (`/Engine/EditorBlueprintResources/StandardMacros.IncrementInt` (`self.WhichInput?`))
    (:`  `
      (set `self.WhichInput?` _result))))

(fn `CheckInput`
  (params (Input :type Text))
  (returns (Image :type "SlateBrush Structure") (TorD :type Boolean))
  (locals (ImageApply :type "SlateBrush Structure" :default (struct :`DrawAs` "Image" :`Tiling` "NoTile" :`Mirroring` "NoMirror" :`ImageType` "NoImage" :`ImageSize` (32.0 32.0) :`Margin` (struct) :`TintColor` (struct :`SpecifiedColor` (struct :`R` 1.0 :`G` 1.0 :`B` 1.0 :`A` 1.0) :`ColorUseRule` "UseColor_Specified") :`OutlineSettings` (struct :`CornerRadii` (struct :`W` 1.0) :`Color` (struct :`SpecifiedColor` (struct) :`ColorUseRule` "UseColor_Specified") :`RoundingType` "HalfHeightRadius") :`ResourceObject` "/Script/Engine.Texture2D'/Game/Mathieu/InteractHuman/Image/I_RightClick.I_RightClick'" :`UVRegion` (struct :`Min` (0.0 0.0) :`Max` (0.0 0.0)))) (LClick :type "SlateBrush Structure" :default (struct :`DrawAs` "Image" :`Tiling` "NoTile" :`Mirroring` "NoMirror" :`ImageType` "NoImage" :`ImageSize` (32.0 32.0) :`Margin` (struct) :`TintColor` (struct :`SpecifiedColor` (struct :`R` 1.0 :`G` 1.0 :`B` 1.0 :`A` 1.0) :`ColorUseRule` "UseColor_Specified") :`OutlineSettings` (struct :`CornerRadii` (struct :`W` 1.0) :`Color` (struct :`SpecifiedColor` (struct) :`ColorUseRule` "UseColor_Specified") :`RoundingType` "HalfHeightRadius") :`ResourceObject` "/Script/Engine.Texture2D'/Game/Mathieu/InteractHuman/Image/I_LeftClick.I_LeftClick'" :`UVRegion` (struct :`Min` (0.0 0.0) :`Max` (0.0 0.0)))) (RClick :type "SlateBrush Structure" :default (struct :`DrawAs` "Image" :`Tiling` "NoTile" :`Mirroring` "NoMirror" :`ImageType` "NoImage" :`ImageSize` (32.0 32.0) :`Margin` (struct) :`TintColor` (struct :`SpecifiedColor` (struct :`R` 1.0 :`G` 1.0 :`B` 1.0 :`A` 1.0) :`ColorUseRule` "UseColor_Specified") :`OutlineSettings` (struct :`CornerRadii` (struct :`W` 1.0) :`Color` (struct :`SpecifiedColor` (struct) :`ColorUseRule` "UseColor_Specified") :`RoundingType` "HalfHeightRadius") :`ResourceObject` "/Script/Engine.Texture2D'/Game/Mathieu/InteractHuman/Image/I_RightClick.I_RightClick'" :`UVRegion` (struct :`Min` (0.0 0.0) :`Max` (0.0 0.0)))) (`TorD?` :type Boolean))
  (switch `string` (`KismetTextLibrary.Conv_TextToString` Input)
    (:`RR`
      (set `local.ImageApply` (`local.RClick`))
      (set `local.TorD?` true))
    (:`LL`
      (set `local.ImageApply` (`local.LClick`))
      (set `local.TorD?` false)))
  (return (`local.ImageApply`) (`local.TorD?`)))

(fn `CreateWidget`
  (params (Image :type "SlateBrush Structure") (`TorD?` :type Boolean) (Speed :type "Float (double-precision)") (LastWidget :type Boolean))
  (locals (Widget :type "/Game/Mathieu/InteractHuman/WB_Qte Object Reference") (TorD :type Boolean) (Im :type "SlateBrush Structure" :default (struct :`DrawAs` "Image" :`Tiling` "NoTile" :`Mirroring` "NoMirror" :`ImageType` "NoImage" :`ImageSize` (32.0 32.0) :`Margin` (struct) :`TintColor` (struct :`SpecifiedColor` (struct :`R` 1.0 :`G` 1.0 :`B` 1.0 :`A` 1.0) :`ColorUseRule` "UseColor_Specified") :`OutlineSettings` (struct :`CornerRadii` (struct :`W` 1.0) :`Color` (struct :`SpecifiedColor` (struct) :`ColorUseRule` "UseColor_Specified") :`RoundingType` "HalfHeightRadius") :`ResourceObject` "/Script/Engine.Texture2D'/Game/Mathieu/InteractHuman/Image/I_RightClick.I_RightClick'" :`UVRegion` (struct :`Min` (0.0 0.0) :`Max` (0.0 0.0)))) (SpeddAnim :type "Float (double-precision)"))
  (bind _widget (`local.Widget`))
  (bind _widget_2 (`local.Widget`))
  (bind _widget_3 (`local.Widget`))
  (set `local.TorD` `TorD?`)
  (set `local.Im` Image)
  (set `local.SpeddAnim` Speed)
  (bind _returnvalue (`|CreateWidget` "/Game/Mathieu/InteractHuman/WB_Qte.WB_Qte_C"))
  (bind _output_get (set `local.Widget` _returnvalue))
  (`KismetArrayLibrary.Array_Add` (`self.WidgetActif?`) _output_get)
  (set `/Game/Mathieu/InteractHuman/WB_Qte.BPQte` self _output_get)
  (set `/Game/Mathieu/InteractHuman/WB_Qte.ImageActive` (`local.TorD`) _widget_2)
  (set `/Game/Mathieu/InteractHuman/WB_Qte.LastWidget?` LastWidget _widget_2)
  (`UserWidget.AddToViewport` _output_get 0)
  (if (`local.TorD`)
    (set `/Game/Mathieu/InteractHuman/WB_Qte.Image0` (`local.Im`) (`local.Widget`))
    (`UserWidget.PlayAnimation` _widget_3 (`/Game/Mathieu/InteractHuman/WB_Qte.AnimT` _widget_3) 0.0 1 "Forward" (`local.SpeddAnim`) false)
    (else
      (set `/Game/Mathieu/InteractHuman/WB_Qte.Image01` (`local.Im`) (`local.Widget`))
      (`UserWidget.PlayAnimation` _widget (`/Game/Mathieu/InteractHuman/WB_Qte.AnimD` _widget) 0.0 1 "Forward" (`local.SpeddAnim`) false))))

(fn `LastWidget`
  (returns (`LasWidget?` :type Boolean))
  (if (== (`KismetArrayLibrary.Array_Length` (`self.QTE_Enum`)) (`self.WhichInput?`))
    (return true)
    (else
      (return false))))

(fn `UserConstructionScript`)